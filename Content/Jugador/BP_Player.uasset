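; BP_Player is the player pawn, handling movement, mouse look and grabbing.
; Axis inputs drive movement along the actor's forward and right vectors, plus controller yaw and pitch scaled by Sensibilidad.
; The forward/back axis alone toggles footstep audio through SoundManager, as its stop check tests that value twice and ignores strafing.
; The Grab input delegates to RaycastAgent.
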(event EventBeginPlay)

(event Collision|EventActorBeginOverlap
  (params (OtherActor :type Actor%20Object%20Reference)))

(event EventTick
  (params (DeltaSeconds :type Float%20%28single-precision%29)))

(event Input|ActionEvents|InputActionGrab
  (params (Key :type Key%20Structure :default "None"))
  ;[1 1 1] RayCast
  (:Pressed
    (Class|RaycastAgent|Grab (Variables|Default|GetRaycastAgent))))

(event Input|AxisEvents|InputAxisAdelante/Atras
  (params (AxisValue :type Float%20%28single-precision%29))
  (bind _soundmanager (Variables|Default|GetSoundManager))
  (bind _audiocomponent (Variables|Default|GetAudioComponent))
  ;[1 1 1] Mover
  (Pawn|Input|AddMovementInput (Transformation|GetActorForwardVector) AxisValue false)
  (Utilities|IsValid (Variables|Default|GetSoundManager)
    (:Is%20Valid
      (if (and (== AxisValue 0.0) (== (stale Input|AxisEvents|InputAxisIzq/Der AxisValue) 0.0))
        (Class|AudioTerrorConfiguration|StopSpawnedSound _soundmanager _audiocomponent)
        (else
          (Class|AudioTerrorConfiguration|PlaySpawnedSound _soundmanager (Variables|Default|GetStepsSoundName) _audiocomponent))))))

(event Input|AxisEvents|InputAxisIzq/Der
  (params (AxisValue :type Float%20%28single-precision%29))
  ;[1 1 1] Mover
  (Pawn|Input|AddMovementInput (Transformation|GetActorRightVector) AxisValue false))

(event Input|AxisEvents|InputAxisMouseX
  (params (AxisValue :type Float%20%28single-precision%29))
  ;[1 1 1] Mover
  (Pawn|Input|AddControllerYawInput (* AxisValue (Variables|Default|GetSensibilidad))))

(event Input|AxisEvents|InputAxisMouseY
  (params (AxisValue :type Float%20%28single-precision%29))
  ;[1 1 1] Mover
  (Pawn|Input|AddControllerPitchInput (* AxisValue (Variables|Default|GetSensibilidad))))

(fn ConstructionScript)