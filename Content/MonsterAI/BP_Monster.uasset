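; BP_Monster is an AI-driven monster that reports the player's proximity to its Blackboard.
; Every Tick, CheckCharacterDistance sets CharacterInRange by testing whether player pawn 0 is within CharacterMinRadius.
; StartBehaviour only calls the empty OnStartBehaviour event.
; The delayed-chase logic is unwired: the TimeUntilFollow timer and the IsChasingMode write never run, and OnStartChasing is empty.
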(event Custom|OnStartChasing
  ;[1 1 1] Timer para comenzar a perseguir
)

(event Custom|OnStartBehaviour
  ;[1 1 1] Timer para comenzar a perseguir
)

(event EventBeginPlay)

(event Collision|EventActorBeginOverlap
  (params (OtherActor :type Actor%20Object%20Reference)))

(event EventTick
  (params (DeltaSeconds :type Float%20%28single-precision%29))
  ;[1 1 1] Revisar la distancia al jugador
  (CallFunction|CheckCharacterDistance))

(fn ConstructionScript)

(fn CheckCharacterDistance
  (AI|Components|Blackboard|SetValueasBool (AI|GetBlackboard 0) (Utilities|Name|MakeLiteralName "CharacterInRange") (<= (Math|Vector|Distance(Vector) (Transformation|GetActorLocation (Game|Player|GetPlayerPawn 0)) (Transformation|GetActorLocation)) (Variables|Default|GetCharacterMinRadius))))

(fn StartBehaviour
  (CallFunction|OnStartBehaviour))